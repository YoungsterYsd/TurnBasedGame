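; BP_floatingNum is a short-lived actor that shows a colored number at a given world location.
; On BeginPlay it passes FloatingNum and SpecifiedColor to the WBP_NumIndicator in its Widget component, then moves itself to TxtLocation with a zero offset.
; It destroys itself after a one-second delay, and the actor's graph applies no motion beyond that initial placement.
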(event `self.ReceiveBeginPlay`
  (bind _aswbp_num_indicator (cast `/Game/_Game/UI/SubUI/WBP_NumIndicator` (`WidgetComponent.GetUserWidgetObject` (`self.Widget`))))
  (`/Game/_Game/UI/SubUI/WBP_NumIndicator.SetIndicatorNum` _aswbp_num_indicator (`self.floatingNum`) (`KismetMathLibrary.Conv_ColorToLinearColor` (`self.specifiedColor`)))
  (bind _output_get (set `self.EndLoc` (+ (`self.txtLocation`) (0.0 0.0 0.0))))
  (`self.K2_SetActorLocation` _output_get)
  (`KismetSystemLibrary.Delay` 1.0)
  (`self.K2_DestroyActor`))

(fn `UserConstructionScript`)